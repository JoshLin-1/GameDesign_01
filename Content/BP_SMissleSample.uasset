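; Missile launcher sample that previews a ballistic arc to the cursor and fires a BP_Missle along it.
; Right-click alternates between showing the aim preview and hiding it to spawn the missile with the computed velocity.
; While the gate is open, cursor updates solve launch velocity, predict the path, rebuild a dashed spline-mesh trail and ease a sphere toward the predicted end.
; Mouse wheel adjusts arc height within limits.
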(event Custom|HidePath
  (bind _returnvalue (Transformation|GetActorLocation))
  (bind _returnvalue_2 (Math|Float|MakeLiteralFloat 0.5))
  (bind _spline (Variables|Default|GetSpline))
  (bind _spline_2 (Variables|Default|GetSpline))
  (bind _sphere (Variables|Default|GetSphere))
  (CallFunction|FnClear)
  (Utilities|FlowControl|Gate true) ; enters at Close
)

(event Custom|ShowPath
  (bind _returnvalue (Transformation|GetActorLocation))
  (bind _returnvalue_2 (Math|Float|MakeLiteralFloat 0.5))
  (bind _spline (Variables|Default|GetSpline))
  (bind _spline_2 (Variables|Default|GetSpline))
  (bind _sphere (Variables|Default|GetSphere))
  (if (Rendering|IsVisible (Variables|Default|GetCursorToWorld))
    (Utilities|FlowControl|Gate true) ; enters at Open
    (else
      (CallFunction|FnClear)
      (Utilities|FlowControl|Gate true) ; enters at Close
    )))

(event EventBeginPlay)

(event Collision|EventActorBeginOverlap
  (params (OtherActor :type Actor%20Object%20Reference)))

(event EventTick
  (params (DeltaSeconds :type Float%20%28single-precision%29))
  (if true
    _))

(event EventRightMouseInteract
  (Utilities|FlowControl|FlipFlop
    (:A
      (Rendering|SetVisibility (Variables|Default|GetSphere) true true)
      (CallFunction|ShowPath))
    (:B
      (Rendering|SetVisibility (Variables|Default|GetSphere) false true)
      (CallFunction|HidePath)
      (bind _returnvalue (Game|SpawnActorfromClass "/Game/BP_Missle.BP_Missle_C" (Transformation|GetWorldTransform (Variables|Default|GetStaticMesh)) "Undefined" 0 0))
      (Variables|/Script/Engine.MovementComponent|SetVelocity (Variables|/Game/BP_Missle.BP_Missle_C|GetProjectileMovement _returnvalue) (Variables|Default|GetVelocity)))))

(event EventInteracttoMousePosition
  (params (CursorPosition :type Vector :default "0, 0, 0"))
  (bind _returnvalue (Transformation|GetActorLocation))
  (bind _returnvalue_2 (Math|Float|MakeLiteralFloat 0.5))
  (bind _spline (Variables|Default|GetSpline))
  (bind _spline_2 (Variables|Default|GetSpline))
  (bind _sphere (Variables|Default|GetSphere))
  (Utilities|FlowControl|Gate true
    (:Exit
      (CallFunction|FnClear)
      (bind _outlaunchvelocity (Game|SuggestProjectileVelocityCustomArc _returnvalue CursorPosition 0.0 (Variables|Default|GetCustomArc)))
      (bind _output_get (Variables|Default|SetVelocity _outlaunchvelocity))
      (bind (_outhit _outpathpositions _outlasttracedestination) (Class|GameplayStatics|BlueprintPredictProjectilePathbyObjectType _returnvalue _output_get true 8e+01 (Utilities|Array|MakeArray "ObjectTypeQuery1") false 0 "None" 0.0 12.0 1e+01))
      (Utilities|FlowControl|Sequence
        (:then_0
          (for (_array_element _array_index) _outpathpositions
            (Spline|AddSplinePointatIndex _spline_2 _array_element _array_index "World" true))
          (Spline|SetSplinePointType _spline_2 (Utilities|Array|LastIndex _outpathpositions) "CurveClamped" true)
          (for _index (range 0 (- (Spline|GetNumberOfSplinePoints _spline_2) 8))
            (bind _returnvalue_3 (AddComponent|AddSplineMeshComponent true))
            (if (not (== (Math|Integer|%(Integer) _index 2) 0))
              (SplineMesh|SetStartScale _returnvalue_3 (Math|Vector2D|MakeVector2D _returnvalue_2 _returnvalue_2) true :!class /Script/Engine.SplineMeshComponent)
              (SplineMesh|SetEndScale _returnvalue_3 (Math|Vector2D|MakeVector2D _returnvalue_2 _returnvalue_2) true :!class /Script/Engine.SplineMeshComponent)
              (Utilities|Array|Add (Variables|Default|GetPoints%20Array) _returnvalue_3)
              (SplineMesh|SetStartandEnd _returnvalue_3 (Utilities|Array|Get(acopy) _outpathpositions _index) (Spline|GetTangentatSplinePoint _spline _index "World") (Utilities|Array|Get(acopy) _outpathpositions (+ _index 1)) (Spline|GetTangentatSplinePoint _spline (+ _index 1) "World") true :!class /Script/Engine.SplineMeshComponent))))
        (:then_1
          (Transformation|SetWorldLocation _sphere (Math|Interpolation|VInterpTo (Transformation|GetWorldLocation _sphere) _outlasttracedestination (Utilities|Time|GetWorldDeltaSeconds) 1e+01) false true))))))

(event EventMouseWhellInteract
  (params (Value :type Float%20%28single-precision%29))
  ;[1 1 1] Wheel Axis
  (if (and (< (Math|Interpolation|FInterptoConstant (Variables|Default|GetCustomArc) (+ (/ Value 1e+01) (Variables|Default|GetCustomArc)) (Utilities|Time|GetWorldDeltaSeconds) 5.0) 0.9) (> (Math|Interpolation|FInterptoConstant (Variables|Default|GetCustomArc) (+ (/ Value 1e+01) (Variables|Default|GetCustomArc)) (Utilities|Time|GetWorldDeltaSeconds) 5.0) 0.1))
    (Variables|Default|SetCustomArc (Math|Interpolation|FInterptoConstant (Variables|Default|GetCustomArc) (+ (/ Value 1e+01) (Variables|Default|GetCustomArc)) (Utilities|Time|GetWorldDeltaSeconds) 5.0))))

(event Input|MouseEvents|MouseWheelAxis
  (params (AxisValue :type Float%20%28single-precision%29)))

(fn ConstructionScript)

(fn FnClear
  (bind _points_array (Variables|Default|GetPoints%20Array))
  (Components|DestroyComponent _points_array)
  (Utilities|Array|Clear _points_array)
  (Spline|ClearSplinePoints (Variables|Default|GetSpline) true))