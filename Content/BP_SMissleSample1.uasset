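; Missile launcher actor with limited ammo that aims through a spawned BP_TargetPoint and fires a BP_Missle along an adjustable arc.
; A looping MultiGate alternates interactions between showing the target point and launching at the cursor position with random spread, using SuggestProjectileVelocityCustomArc.
; The mouse wheel adjusts the arc, Tick cancels aiming when CursorToWorld is hidden, and SGameModeBase tracks total ammo.
; Older in-actor spline trajectory preview logic remains disconnected.
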(event Custom|HidePath)

(event Custom|ShowPath)

(event EventBeginPlay
  (bind _assgame_mode_base (Utilities|Casting|CastToSGameModeBase (Game|GetGameMode)))
  (Variables|/Game/SGameModeBase.SGameModeBase_C|SetGetAllBullet _assgame_mode_base (+ (Variables|/Game/SGameModeBase.SGameModeBase_C|GetGetAllBullet _assgame_mode_base) (Variables|Default|GetBullet))))

(event Collision|EventActorBeginOverlap
  (params (OtherActor :type Actor%20Object%20Reference)))

(event EventTick
  (params (DeltaSeconds :type Float%20%28single-precision%29))
  (bind _staticmesh (Variables|Default|GetStaticMesh))
  (bind _max (Variables|Default|GetMax))
  (bind _min (Variables|Default|GetMin))
  (bind _returnvalue (Transformation|GetWorldTransform _staticmesh))
  (if (not (Rendering|IsVisible (Variables|Default|GetCursorToWorld)))
    (Utilities|IsValid (stale EventInteracttoMousePosition _returnvalue_2)
      (:Is%20Valid
        (Default|HidePath (stale EventInteracttoMousePosition _returnvalue_2))
        (Actor|DestroyActor (stale EventInteracttoMousePosition _returnvalue_2))
        (Utilities|FlowControl|MultiGate false true -1) ; enters at Reset
      ))))

(event EventInteracttoMousePosition
  (params (CursorPosition :type Vector :default "0, 0, 0"))
  (bind _staticmesh (Variables|Default|GetStaticMesh))
  (bind _max (Variables|Default|GetMax))
  (bind _min (Variables|Default|GetMin))
  (bind _returnvalue (Transformation|GetWorldTransform _staticmesh))
  (if (> (Variables|Default|GetBullet) 0.0)
    (Utilities|FlowControl|MultiGate false true -1
      (:Out%200
        (bind _returnvalue_2 (Game|SpawnActorfromClass "/Game/BP_TargetPoint.BP_TargetPoint_C" _returnvalue "Undefined" 0 0))
        (Default|ShowPath _returnvalue_2)
        (Variables|Default|SetTargetPoint _returnvalue_2))
      (:Out%201
        (Default|HidePath _returnvalue_2)
        (Actor|DestroyActor _returnvalue_2)
        (bind _outlaunchvelocity (Game|SuggestProjectileVelocityCustomArc (Transformation|GetActorLocation) (+ CursorPosition (Math|Vector|MakeVector (Math|Random|RandomFloatinRange _min _max) (Math|Random|RandomFloatinRange _min _max) 0.0)) 0.0 (Variables|Default|GetCustomArc)))
        (bind _returnvalue_3 (Game|SpawnActorfromClass "/Game/BP_Missle.BP_Missle_C" _returnvalue "Undefined" 0 0))
        (Variables|/Script/Engine.MovementComponent|SetVelocity (Variables|/Game/BP_Missle.BP_Missle_C|GetProjectileMovement _returnvalue_3) _outlaunchvelocity)
        (Variables|Default|SetBullet (- (Variables|Default|GetBullet) 1.0))
        (bind _assgame_mode_base (Utilities|Casting|CastToSGameModeBase (Game|GetGameMode)))
        (Variables|/Game/SGameModeBase.SGameModeBase_C|SetGetAllBullet _assgame_mode_base (- (Variables|/Game/SGameModeBase.SGameModeBase_C|GetGetAllBullet _assgame_mode_base) 1.0))))))

(event EventMouseWhellInteract
  (params (Value :type Float%20%28single-precision%29))
  (bind _targetpoint (Variables|Default|GetTargetPoint))
  ;[1 1 1] Wheel Axis
  (if (and (< (Math|Interpolation|FInterptoConstant (Variables|Default|GetCustomArc) (+ (/ Value 1e+01) (Variables|Default|GetCustomArc)) (Utilities|Time|GetWorldDeltaSeconds) 5.0) 0.9) (> (Math|Interpolation|FInterptoConstant (Variables|Default|GetCustomArc) (+ (/ Value 1e+01) (Variables|Default|GetCustomArc)) (Utilities|Time|GetWorldDeltaSeconds) 5.0) 0.1))
    (bind _output_get (Variables|Default|SetCustomArc (Math|Interpolation|FInterptoConstant (Variables|Default|GetCustomArc) (+ (/ Value 1e+01) (Variables|Default|GetCustomArc)) (Utilities|Time|GetWorldDeltaSeconds) 5.0)))
    (Utilities|IsValid _targetpoint
      (:Is%20Valid
        (Variables|/Game/BP_TargetPoint.BP_TargetPoint_C|SetCustom%20Arc _targetpoint _output_get)))))

(fn ConstructionScript)

(fn FnClear
  (bind _points_array (Variables|Default|GetPoints%20Array))
  (Components|DestroyComponent _points_array)
  (Utilities|Array|Clear _points_array))