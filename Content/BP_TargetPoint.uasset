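; BP_TargetPoint draws a dashed projectile-arc preview from the actor toward the practice player controller's mouse position.
; ShowPath and HidePath toggle a Tick gate that clears and rebuilds the preview each frame from a suggested arc velocity and predicted path.
; Path points feed a spline, with odd-indexed segments drawn as half-scale spline meshes, stopping short of the end.
; A sphere eases toward the predicted trace destination.
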(event Custom|HidePath
  (bind _returnvalue (Math|Float|MakeLiteralFloat 0.5))
  (bind _returnvalue_2 (Transformation|GetActorLocation))
  (bind _spline (Variables|Default|GetSpline))
  (bind _spline_2 (Variables|Default|GetSpline))
  (bind _sphere (Variables|Default|GetSphere))
  (CallFunction|FnClear)
  (Utilities|FlowControl|Gate true) ; enters at Close
)

(event Custom|ShowPath
  (bind _returnvalue (Math|Float|MakeLiteralFloat 0.5))
  (bind _returnvalue_2 (Transformation|GetActorLocation))
  (bind _spline (Variables|Default|GetSpline))
  (bind _spline_2 (Variables|Default|GetSpline))
  (bind _sphere (Variables|Default|GetSphere))
  (Utilities|FlowControl|Gate true) ; enters at Open
)

(event EventTick
  (params (DeltaSeconds :type Float%20%28single-precision%29))
  (bind _returnvalue (Math|Float|MakeLiteralFloat 0.5))
  (bind _returnvalue_2 (Transformation|GetActorLocation))
  (bind _spline (Variables|Default|GetSpline))
  (bind _spline_2 (Variables|Default|GetSpline))
  (bind _sphere (Variables|Default|GetSphere))
  (bind _asbp_practice_player_controller (Utilities|Casting|CastToBP_PracticePlayerController (Game|GetPlayerController 0)))
  (Utilities|FlowControl|Gate true
    (:Exit
      (CallFunction|FnClear)
      (bind _outlaunchvelocity (Game|SuggestProjectileVelocityCustomArc _returnvalue_2 (Variables|/Game/BP_PracticePlayerController.BP_PracticePlayerController_C|GetMouse%20Position _asbp_practice_player_controller) 0.0 (Variables|Default|GetCustom%20Arc)))
      (bind (_outhit _outpathpositions _outlasttracedestination) (Class|GameplayStatics|BlueprintPredictProjectilePathbyObjectType _returnvalue_2 _outlaunchvelocity true 8e+01 (Utilities|Array|MakeArray "ObjectTypeQuery1") false 0 "None" 0.0 12.0 1e+01))
      (Utilities|FlowControl|Sequence
        (:then_0
          (for (_array_element _array_index) _outpathpositions
            (Spline|AddSplinePointatIndex _spline _array_element _array_index "World" true))
          (Spline|SetSplinePointType _spline (Utilities|Array|LastIndex _outpathpositions) "CurveClamped" true)
          (for _index (range 0 (- (Spline|GetNumberOfSplinePoints _spline) 8))
            (bind _returnvalue_3 (AddComponent|AddSplineMeshComponent true))
            (if (not (== (Math|Integer|%(Integer) _index 2) 0))
              (SplineMesh|SetStartScale _returnvalue_3 (Math|Vector2D|MakeVector2D _returnvalue _returnvalue) true :!class /Script/Engine.SplineMeshComponent)
              (SplineMesh|SetEndScale _returnvalue_3 (Math|Vector2D|MakeVector2D _returnvalue _returnvalue) true :!class /Script/Engine.SplineMeshComponent)
              (Utilities|Array|Add (Variables|Default|GetPoints%20Array) _returnvalue_3)
              (SplineMesh|SetStartandEnd _returnvalue_3 (Utilities|Array|Get(acopy) _outpathpositions _index) (Spline|GetTangentatSplinePoint _spline_2 _index "World") (Utilities|Array|Get(acopy) _outpathpositions (+ _index 1)) (Spline|GetTangentatSplinePoint _spline_2 (+ _index 1) "World") true :!class /Script/Engine.SplineMeshComponent))))
        (:then_1
          (Transformation|SetWorldLocation _sphere (Math|Interpolation|VInterpTo (Transformation|GetWorldLocation _sphere) _outlasttracedestination (Utilities|Time|GetWorldDeltaSeconds) 1e+01) false true))))))

(fn ConstructionScript)

(fn FnClear
  (bind _points_array (Variables|Default|GetPoints%20Array))
  (Components|DestroyComponent _points_array)
  (Utilities|Array|Clear _points_array)
  (Spline|ClearSplinePoints (Variables|Default|GetSpline) true))