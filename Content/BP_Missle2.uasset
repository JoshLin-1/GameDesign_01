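; Rocket launcher Blueprint that previews a missile's arc before firing it from the holder's mouth socket.
; E alternately shows the preview, or hides it and spawns BP_Missle with the previewed velocity.
; While shown, Tick rebuilds a predicted projectile path as alternating spline mesh segments for a dashed line, easing a sphere toward the predicted endpoint.
; The mouse wheel adjusts Direction within limits, scaling launch speed along the socket's forward vector.
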(event Custom|HidePath
  (bind _returnvalue (Math|Float|MakeLiteralFloat 0.5))
  (bind _rokcet_holder (Variables|Default|GetRokcet_Holder))
  (bind _sphere (Variables|Default|GetSphere))
  (bind _spline (Variables|Default|GetSpline))
  (bind _spline_2 (Variables|Default|GetSpline))
  (bind _direction (Variables|Default|GetDirection))
  (bind _speed (Variables|Default|GetSpeed))
  (bind _returnvalue_2 (Transformation|GetSocketTransform _rokcet_holder "Mouth" "RTS_World"))
  (bind _returnvalue_3 (Math|Vector|GetForwardVector (.rotation _returnvalue_2)))
  (bind _returnvalue_4 (* _returnvalue_3 _direction))
  (bind _returnvalue_5 (+ _returnvalue_3 _returnvalue_4))
  (bind _returnvalue_6 (* _returnvalue_5 _speed))
  (CallFunction|FnClear)
  (Utilities|FlowControl|Gate true) ; enters at Close
)

(event Custom|ShowPath
  (bind _returnvalue (Math|Float|MakeLiteralFloat 0.5))
  (bind _rokcet_holder (Variables|Default|GetRokcet_Holder))
  (bind _sphere (Variables|Default|GetSphere))
  (bind _spline (Variables|Default|GetSpline))
  (bind _spline_2 (Variables|Default|GetSpline))
  (bind _direction (Variables|Default|GetDirection))
  (bind _speed (Variables|Default|GetSpeed))
  (bind _returnvalue_2 (Transformation|GetSocketTransform _rokcet_holder "Mouth" "RTS_World"))
  (bind _returnvalue_3 (Math|Vector|GetForwardVector (.rotation _returnvalue_2)))
  (bind _returnvalue_4 (* _returnvalue_3 _direction))
  (bind _returnvalue_5 (+ _returnvalue_3 _returnvalue_4))
  (bind _returnvalue_6 (* _returnvalue_5 _speed))
  (Utilities|FlowControl|Gate true) ; enters at Open
)

(event EventTick
  (params (DeltaSeconds :type Float%20%28single-precision%29))
  (bind _returnvalue (Math|Float|MakeLiteralFloat 0.5))
  (bind _rokcet_holder (Variables|Default|GetRokcet_Holder))
  (bind _sphere (Variables|Default|GetSphere))
  (bind _spline (Variables|Default|GetSpline))
  (bind _spline_2 (Variables|Default|GetSpline))
  (bind _direction (Variables|Default|GetDirection))
  (bind _speed (Variables|Default|GetSpeed))
  (bind _returnvalue_2 (Transformation|GetSocketTransform _rokcet_holder "Mouth" "RTS_World"))
  (bind _returnvalue_3 (Math|Vector|GetForwardVector (.rotation _returnvalue_2)))
  (bind _returnvalue_4 (* _returnvalue_3 _direction))
  (bind _returnvalue_5 (+ _returnvalue_3 _returnvalue_4))
  (bind _returnvalue_6 (* _returnvalue_5 _speed))
  (Utilities|FlowControl|Gate true
    (:Exit
      (CallFunction|FnClear)
      (Variables|Default|SetMissleVelocity _returnvalue_6)
      (bind (_outhit _outpathpositions _outlasttracedestination) (Class|GameplayStatics|BlueprintPredictProjectilePathbyObjectType (.location _returnvalue_2) _returnvalue_6 true 8e+01 (Utilities|Array|MakeArray "ObjectTypeQuery1") false 0 "None" 0.0 12.0 1e+01))
      (Utilities|FlowControl|Sequence
        (:then_0
          (for (_array_element _array_index) _outpathpositions
            (Spline|AddSplinePointatIndex _spline _array_element _array_index "World" true))
          (Spline|SetSplinePointType _spline (Utilities|Array|LastIndex _outpathpositions) "CurveClamped" true)
          (for _index (range 0 (- (Spline|GetNumberOfSplinePoints _spline) 8))
            (bind _returnvalue_7 (AddComponent|AddSplineMeshComponent true))
            (if (== (Math|Integer|%(Integer) _index 2) 0)
              (SplineMesh|SetStartScale _returnvalue_7 (Math|Vector2D|MakeVector2D _returnvalue _returnvalue) true :!class /Script/Engine.SplineMeshComponent)
              (SplineMesh|SetEndScale _returnvalue_7 (Math|Vector2D|MakeVector2D _returnvalue _returnvalue) true :!class /Script/Engine.SplineMeshComponent)
              (Utilities|Array|Add (Variables|Default|GetPointArray) _returnvalue_7)
              (SplineMesh|SetStartandEnd _returnvalue_7 (Utilities|Array|Get(acopy) _outpathpositions _index) (Spline|GetTangentatSplinePoint _spline_2 _index "World") (Utilities|Array|Get(acopy) _outpathpositions (+ _index 1)) (Spline|GetTangentatSplinePoint _spline_2 (+ _index 1) "World") true :!class /Script/Engine.SplineMeshComponent))))
        (:then_1
          (Transformation|SetWorldLocation _sphere (Math|Interpolation|VInterpTo (Transformation|GetWorldLocation _sphere) _outlasttracedestination (Utilities|Time|GetWorldDeltaSeconds) 1e+01) false true))))))

(event Input|MouseEvents|MouseWheelAxis
  (params (AxisValue :type Float%20%28single-precision%29))
  ;[1 1 1] Wheel Axis
  (if (and (< (Math|Interpolation|FInterptoConstant (Variables|Default|GetDirection) (+ (/ AxisValue 1e+01) (Variables|Default|GetDirection)) (Utilities|Time|GetWorldDeltaSeconds) 5.0) 0.7) (> (Math|Interpolation|FInterptoConstant (Variables|Default|GetDirection) (+ (/ AxisValue 1e+01) (Variables|Default|GetDirection)) (Utilities|Time|GetWorldDeltaSeconds) 5.0) -0.4))
    (Variables|Default|SetDirection (Math|Interpolation|FInterptoConstant (Variables|Default|GetDirection) (+ (/ AxisValue 1e+01) (Variables|Default|GetDirection)) (Utilities|Time|GetWorldDeltaSeconds) 5.0))))

(event Input|KeyboardEvents|E
  (params (Key :type Key%20Structure :default "None"))
  ;[1 1 1] Turn On and Off
  (:Pressed
    (Utilities|FlowControl|FlipFlop
      (:A
        (Rendering|SetVisibility (Variables|Default|GetSphere) true true)
        (CallFunction|ShowPath))
      (:B
        (Rendering|SetVisibility (Variables|Default|GetSphere) false true)
        (CallFunction|HidePath)
        (bind _returnvalue (Game|SpawnActorfromClass "/Game/BP_Missle.BP_Missle_C" (Transformation|GetSocketTransform (Variables|Default|GetRokcet_Holder) "mouth" "RTS_World") "Undefined" 0 0))
        (Variables|/Script/Engine.MovementComponent|SetVelocity (Variables|/Game/BP_Missle.BP_Missle_C|GetProjectileMovement _returnvalue) (Variables|Default|GetMissleVelocity))))))

(fn ConstructionScript)

(fn FnClear
  (bind _pointarray (Variables|Default|GetPointArray))
  (Components|DestroyComponent _pointarray)
  (Utilities|Array|Clear _pointarray)
  (Spline|ClearSplinePoints (Variables|Default|GetSpline) true))